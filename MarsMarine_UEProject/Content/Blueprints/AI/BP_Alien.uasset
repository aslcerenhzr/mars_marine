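; BP_Alien is an enemy that repeatedly chases the player with AIMoveTo.
; Within AttackRange it halts movement for an attack montage; DamagePlayer applies damage but is not called here.
; Any damage kills it, as DecreasesHealth always returns zero and subtracts DamagePerHit instead of incoming Damage.
; Death disables movement and collision, credits BP_Marine's kills, notifies BP_GameMode, then destroys the actor after a delay.
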(event `self.ReceiveBeginPlay`
  (if (not (`self.Dead`))
    (`|AIMoveTo` self (0.0 0.0 0.0) (`GameplayStatics.GetPlayerCharacter` 0) :!label _label
      (:`OnSuccess`
        _)
      (:`OnFail`
        _))
    (`KismetSystemLibrary.Delay` 0.2)
    (goto _label)))

(event `self.ReceiveTick`
  (params (DeltaSeconds :type "Float (single-precision)"))
  (if (and (`self.Is Within Attack Range`) (not (`self.Is Attacking`)))
    (if (not (`self.Dead`))
      (`ActorComponent.Deactivate` (`self.CharacterMovement`))
      (`|PlayMontage` (`self.Mesh`) "/Game/Characters/Enemy_Great_Spider/Animations/AlienAttack1.AlienAttack1"
        (:`OnCompleted`
          (`ActorComponent.Activate` (`self.CharacterMovement`) false))))))

(event `self.ReceiveAnyDamage`
  (params (Damage :type "Float (single-precision)") (DamageType :type "DamageType Object Reference") (InstigatedBy :type "Controller Object Reference") (DamageCauser :type "Actor Object Reference"))
  (if (not (`self.Dead`))
    (bind _ailen_s_health (`self.Decreases Health` Damage))
    (if (== _ailen_s_health 0.0)
      (`self.Kill AI`)
      (`KismetSystemLibrary.Delay` 3.0)
      (`self.K2_DestroyActor`))))

(fn `Damage Player`
  (`GameplayStatics.ApplyDamage` (`GameplayStatics.GetPlayerCharacter` 0) (`self.Damage Per Hit`)))

(fn `Decreases Health`
  (params (Damage :type "Float (double-precision)"))
  (returns (`Ailen's Health` :type "Float (double-precision)"))
  (set `self.Ailen's Health` (`KismetMathLibrary.FClamp` (- (`self.Ailen's Health`) (`self.Damage Per Hit`)) 0.0 100.0))
  (return 0.0))

(fn `Is Attacking`
  (returns (`return value` :type Boolean))
  (return (`AnimInstance.Montage_IsPlaying` (`SkeletalMeshComponent.GetAnimInstance` (`self.Mesh`)) "/Game/Characters/Enemy_Great_Spider/Animations/AlienAttack1.AlienAttack1")))

(fn `Is Within Attack Range`
  (returns (NewParam :type Boolean))
  (return (<= (`self.GetDistanceTo` (`GameplayStatics.GetPlayerCharacter` 0)) (`self.Attack Range`))))

(fn `Kill AI`
  (bind _charactermovement (`self.CharacterMovement`))
  (set `self.Dead` true)
  (`MovementComponent.StopMovementImmediately` _charactermovement)
  (`ActorComponent.Deactivate` _charactermovement)
  (`self.SetActorEnableCollision` false)
  (bind _asbp_marine (cast `/Game/Blueprints/Pawns/BP_Marine` (`GameplayStatics.GetPlayerCharacter` 0)))
  (`/Game/Blueprints/Pawns/BP_Marine.Increase Kills` _asbp_marine)
  (bind _asbp_game_mode (cast `/Game/Blueprints/BP_GameMode` (`GameplayStatics.GetGameMode`)))
  (`/Game/Blueprints/BP_GameMode.Register Alien Death` _asbp_game_mode self))

(fn `UserConstructionScript`)